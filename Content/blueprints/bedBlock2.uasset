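; Interactable block actor that becomes a heavy physics object when the player presses E nearby.
; Box overlap with the player character enables input on the actor, and leaving the box disables it.
; The E press raises the StaticMesh mass scale and turns on physics simulation, with no logic to reverse either.
; Falllocation is unused.
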(event `Key|E`
  (params (Key :type "Key Structure"))
  (:`Pressed`
    (`PrimitiveComponent.SetMassScale` (`self.StaticMesh`) "None" 200.0)
    (`PrimitiveComponent.SetSimulatePhysics` (`self.StaticMesh`) true)))

(event `self.Box.OnComponentBeginOverlap`
  (params (OverlappedComponent :type "PrimitiveComponent Object Reference") (OtherActor :type "Actor Object Reference") (OtherComp :type "PrimitiveComponent Object Reference") (OtherBodyIndex :type Integer) (bFromSweep :type Boolean) (SweepResult :type "HitResult Structure (by ref)"))
  (if (== OtherActor (`GameplayStatics.GetPlayerCharacter` 0))
    (`self.EnableInput` (`GameplayStatics.GetPlayerController` 0))))

(event `self.Box.OnComponentEndOverlap`
  (params (OverlappedComponent :type "PrimitiveComponent Object Reference") (OtherActor :type "Actor Object Reference") (OtherComp :type "PrimitiveComponent Object Reference") (OtherBodyIndex :type Integer))
  (if (== OtherActor (`GameplayStatics.GetPlayerCharacter` 0))
    (`self.DisableInput` (`GameplayStatics.GetPlayerController` 0))))

(fn `UserConstructionScript`)